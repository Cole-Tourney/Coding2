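; BP_Wallcandlestick_B is a configurable wall candlestick prop with a point light and a candle fire effect.
; Its construction script applies the Lumens, Radius and Temperature variables to the light's intensity, attenuation radius and temperature.
; RemoveLight and RemoveFX flags destroy the light or fire component during construction.
; The event graph holds only disabled placeholder events, so the Blueprint adds no runtime logic.
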(fn `UserConstructionScript`
  (bind _pointlight (`self.PointLight`))
  (`|ExecutionSequence`
    (:`then_0`
      (`LightComponent.SetIntensity` _pointlight (`self.Lumens`))
      (`LocalLightComponent.SetAttenuationRadius` _pointlight (`self.Radius`))
      (`LightComponent.SetTemperature` _pointlight (`self.Temperature`)))
    (:`then_1`
      (if (`self.Remove Light`)
        (`ActorComponent.K2_DestroyComponent` (`self.PointLight`))))
    (:`then_2`
      (if (`self.Remove FX`)
        (`ActorComponent.K2_DestroyComponent` (`self.FX_Candle_Fire_A`))))))