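; BP_Cole_Door is a key-locked door that opens when the player interacts while holding enough keys.
; Interact checks the third-person character's KeyCount against KeysNeeded, deducts that cost, flags the door unlocked and prints the remaining count.
; A timeline then lerps the door downward from its starting location and destroys the actor when finished.
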(event `/Game/Cole/Blueprints/BPI_Interact.Interact`
  (bind (_doorstartinglocation_x _doorstartinglocation_y _doorstartinglocation_z) (`KismetMathLibrary.BreakVector` (`self.doorStartingLocation`)))
  (bind _asbp_third_person_character (cast `/Game/ThirdPerson/Blueprints/BP_ThirdPersonCharacter` (`GameplayStatics.GetPlayerCharacter` 0)))
  (if (>= (`/Game/ThirdPerson/Blueprints/BP_ThirdPersonCharacter.keyCount` _asbp_third_person_character) (`self.keysNeeded`))
    (set `self.doorUnlocked` true)
    (bind _output_get (set `/Game/ThirdPerson/Blueprints/BP_ThirdPersonCharacter.keyCount` (- (`/Game/ThirdPerson/Blueprints/BP_ThirdPersonCharacter.keyCount` _asbp_third_person_character) (`self.keysNeeded`)) _asbp_third_person_character))
    (set `self.doorStartingLocation` (`self.K2_GetActorLocation`))
    (`KismetSystemLibrary.PrintString` (`KismetStringLibrary.Concat_StrStr` "player has " (`KismetStringLibrary.Conv_IntToString` _output_get) " keys"))
    (bind (_direction _newtrack_0) (`Timeline|Timeline`)
      (:`Update`
        (`self.K2_SetActorRelativeLocation` (`KismetMathLibrary.MakeVector` _doorstartinglocation_x _doorstartinglocation_y (`KismetMathLibrary.Lerp` _doorstartinglocation_z (+ _doorstartinglocation_z -400.0) _newtrack_0))))
      (:`Finished`
        (`self.K2_DestroyActor`)))))

(fn `UserConstructionScript`)