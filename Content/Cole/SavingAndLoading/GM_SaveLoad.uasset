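; GameMode that saves and restores per-level state, using the current level's name as the save slot.
; On BeginPlay it loads the slot's SG_LevelState, or creates a new one if none exists.
; After loading, it calls CollectThyself on each valid entry in the saved CollectedCoins array to reapply pickups.
; SaveLevelStateToFile writes that same object back to the slot and prints whether the save succeeded.
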(event `self.ReceiveBeginPlay`
  (`self.LoadLevelStateFromFile`))

(event `SaveLevelStateToFile`
  (bind _returnvalue (`GameplayStatics.GetCurrentLevelName` true))
  (bind _returnvalue_2 (`GameplayStatics.SaveGameToSlot` (`self.SG_LevelState`) _returnvalue))
  (if _returnvalue_2
    (`KismetSystemLibrary.PrintText` "Level State Saved" true true (struct :`R` 0.130028 :`G` 1.0 :`B` 0.152271 :`A` 1.0) 5.0)
    (else
      (`KismetSystemLibrary.PrintText` "Failed to Save" true true (struct :`R` 1.0 :`G` 0.040042 :`B` 0.023332 :`A` 1.0) 5.0))))

(event `LoadLevelStateFromFile`
  (bind _returnvalue (`GameplayStatics.GetCurrentLevelName` true))
  (bind _returnvalue_2 (`GameplayStatics.DoesSaveGameExist` _returnvalue))
  (if _returnvalue_2
    (bind _returnvalue_3 (`GameplayStatics.LoadGameFromSlot` _returnvalue))
    (bind _assg_level_state (cast `/Game/Cole/SavingAndLoading/SG_LevelState` _returnvalue_3))
    (set `self.SG_LevelState` _assg_level_state)
    (for _array_element (`/Game/Cole/SavingAndLoading/SG_LevelState.collectedCoins` (`self.SG_LevelState`))
      (`/Engine/EditorBlueprintResources/StandardMacros.IsValid` _array_element
        (:`Is Valid`
          (`/Game/Cole/Blueprints/BP_Coin.CollectThyself` _array_element))))
    (else
      (bind _returnvalue_4 (`GameplayStatics.CreateSaveGameObject` "/Game/Cole/SavingAndLoading/SG_LevelState.SG_LevelState_C"))
      (set `self.SG_LevelState` _returnvalue_4))))

(fn `UserConstructionScript`)