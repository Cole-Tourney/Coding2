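; BP_PatrolRoute is a patrol route that serves world-space patrol point locations from a spline, one per call.
; GetPatrolPointLocation steps PatrolIndex by Direction, then returns that spline point's location.
; Direction flips at either end for back-and-forth traversal, though the upper flip waits until the index reaches the point count, one past the last valid index.
; The event graph and construction script are empty.
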(fn `GetPatrolPointLocation`
  (returns (ReturnValue :type "Vector Structure"))
  (bind _patrolindex (`self.patrolIndex`))
  (set `self.patrolIndex` (+ (`self.Direction`) (`self.patrolIndex`)))
  (if (>= _patrolindex (`SplineComponent.GetNumberOfSplinePoints` (`self.Spline`)))
    (set `self.Direction` -1)
    (elif (<= _patrolindex 0)
      (set `self.Direction` 1)))
  (return (`SplineComponent.GetLocationAtSplinePoint` (`self.Spline`) (`self.patrolIndex`) "World")))

(fn `UserConstructionScript`)