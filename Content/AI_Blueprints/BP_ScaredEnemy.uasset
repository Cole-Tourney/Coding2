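; BP_ScaredEnemy is an AI enemy character that patrols, attacks with a left-hook montage and ragdolls when its health runs out.
; It exposes walk speed, attack and strafe ranges, and aggro toggles that swap its material to flat red.
; Patrol points ping-pong along a spline route, and attacks signal AttackFinished on completion or interruption.
; Point damage reduces health, then triggers physics with a radial impulse on death.
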(event `Attack`
  (`KismetSystemLibrary.PrintText` "Attack!!")
  (`|PlayMontage` (`self.Mesh`) "/Game/CloseCombatAnimSet/Animations/InPlace/Attacks/AM_LeftHook.AM_LeftHook"
    (:`OnCompleted`
      _)
    (:`OnInterrupted`
      _))
  (`self.AttackFinished`))

(event `self.ReceiveBeginPlay`
  (set `self.OriginalMaterial` (`PrimitiveComponent.GetMaterial` (`self.Mesh`) 0)))

(event `GetAggro`
  (`PrimitiveComponent.SetMaterial` (`self.Mesh`) 0 "/Game/Materials/MI_FlatRed.MI_FlatRed")
  (set `self.Aggroed` true))

(event `LoseAggro`
  (`PrimitiveComponent.SetMaterial` (`self.Mesh`) 0 (`self.OriginalMaterial`))
  (set `self.Aggroed` false))

(event `Set Walk Speed`
  (params (Speed :type "Float (single-precision)" :default 400.0))
  (set `CharacterMovementComponent.MaxWalkSpeed` Speed (`self.CharacterMovement`)))

(event `self.ReceivePointDamage`
  (params (Damage :type "Float (single-precision)") (DamageType :type "DamageType Object Reference") (HitLocation :type "Vector Structure") (HitNormal :type "Vector Structure") (HitComponent :type "PrimitiveComponent Object Reference") (BoneName :type Name) (ShotFromDirection :type "Vector Structure") (InstigatedBy :type "Controller Object Reference") (DamageCauser :type "Actor Object Reference") (HitInfo :type "HitResult Structure (by ref)"))
  (`KismetSystemLibrary.PrintText` (`|FormatText` "{Instigator} Hit me for {damage} damage" InstigatedBy Damage))
  (bind _output_get (set `self.Health` (- (`self.Health`) Damage)))
  (`KismetSystemLibrary.PrintText` (`|FormatText` "Current Health: {health}" (`KismetTextLibrary.Conv_DoubleToText` _output_get "HalfToEven")))
  (if (<= (`self.Health`) 0.0)
    (`KismetSystemLibrary.PrintText` "I diead")
    (`self.Ragdoll` ShotFromDirection)))

(event `Ragdoll`
  (params (Origin :type "Vector Structure"))
  (bind _mesh (`self.Mesh`))
  (`PrimitiveComponent.SetSimulatePhysics` _mesh true)
  (`PrimitiveComponent.AddRadialImpulse` _mesh (+ Origin (0.0 0.0 0.0)) 300.0 30000.0 "RIF_Constant" false)
  (`CharacterMovementComponent.DisableMovement` (`self.CharacterMovement`)))

(fn `GetIdealRange`
  (returns (AttackRange :type "Float (double-precision)") (StrafeRange :type "Float (double-precision)"))
  (return (`self.Attack Range`) (`self.Strafe Range`)))

(fn `GetPatrolPointLocation`
  (returns (ReturnValue :type "Vector Structure"))
  (bind _patrolindex (`self.patrolIndex`))
  (set `self.patrolIndex` (+ (`self.Direction`) (`self.patrolIndex`)))
  (if (>= _patrolindex (- (`SplineComponent.GetNumberOfSplinePoints` (`/Game/AI_Blueprints/BP_PatrolRoute.Spline` (`self.PatrolRoute`))) 1))
    (set `self.Direction` -1)
    (elif (<= _patrolindex 0)
      (set `self.Direction` 1)))
  (return (`SplineComponent.GetLocationAtSplinePoint` (`/Game/AI_Blueprints/BP_PatrolRoute.Spline` (`self.PatrolRoute`)) (`self.patrolIndex`) "World")))

(fn `UserConstructionScript`)